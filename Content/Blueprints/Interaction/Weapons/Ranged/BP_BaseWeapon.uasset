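; Base VR ranged weapon that is grabbed by motion controllers through a physics handle and fired on Use.
; A second grabbing hand becomes SecondaryHand, and Tick rotates the mesh from the primary hand toward it.
; Overlapping Mag_Trigger with matching ammo snaps it in as the magazine, and ending the overlap detaches it.
; Fire plays muzzle effects, spends a round and returns a debug-drawn line trace hit without applying damage.
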(event `self.ReceiveTick`
  (params (DeltaSeconds :type "Float (single-precision)"))
  (`self.RotateWeapon`))

(event `/Game/Blueprints/FunctionsAndInterfaces/BP_InteractionInterface.GrabItem`
  (params (PhysicsHandle :type "PhysicsHandleComponent Object Reference") (MC :type "/Game/Blueprints/Player/BP_MotionController Object Reference"))
  (bind _primholding (`self.PrimHolding`))
  (bind (_returnvalue_location _returnvalue_rotation) (`KismetMathLibrary.BreakTransform` (`SceneComponent.K2_GetComponentToWorld` (`/Game/Blueprints/Player/BP_MotionController.MotionController` MC))))
  (if (== _primholding null)
    (set `self.GrabPhys` PhysicsHandle)
    (if (`self.SnapToController`)
      (`self.K2_SetActorRotation` (`SceneComponent.K2_GetComponentRotation` (`/Game/Blueprints/Player/BP_MotionController.Sphere` MC))))
    (`PhysicsHandleComponent.GrabComponentAtLocationWithRotation` PhysicsHandle (`self.BaseMesh`) "None" _returnvalue_location _returnvalue_rotation)
    (set `self.PrimHolding` MC)
    (elif (not (== MC _primholding))
      (set `self.SecondaryHand` MC))))

(event `/Game/Blueprints/FunctionsAndInterfaces/BP_InteractionInterface.DropItem`
  (params (PhysicsHandle :type "PhysicsHandleComponent Object Reference") (MC :type "/Game/Blueprints/Player/BP_MotionController Object Reference"))
  (bind _secondaryhand (`self.SecondaryHand`))
  ;[1 1 1] Drop
  (`/Engine/EditorBlueprintResources/StandardMacros.IsValid` _secondaryhand
    (:`Is Valid`
      (if (== MC _secondaryhand)
        (set `self.SecondaryHand` null)))
    (:`Is Not Valid`
      (`self.Drop` PhysicsHandle)
      (set `self.PrimHolding` null))))

(event `/Game/Blueprints/FunctionsAndInterfaces/BP_InteractionInterface.Use`
  (`self.Fire`))

(event `self.Mag_Trigger.OnComponentBeginOverlap`
  (params (OverlappedComponent :type "PrimitiveComponent Object Reference") (OtherActor :type "Actor Object Reference") (OtherComp :type "PrimitiveComponent Object Reference") (OtherBodyIndex :type Integer) (bFromSweep :type Boolean) (SweepResult :type "HitResult Structure (by ref)"))
  ;[1 1 1] Attach Mag
  (bind _asbp_ammo_base (cast `/Game/Blueprints/Interaction/Weapons/Ranged/Ammo/BP_AmmoBase` OtherActor))
  (if (== (`/Game/Blueprints/Interaction/Weapons/Ranged/Ammo/BP_AmmoBase.AmmoType` _asbp_ammo_base) (`self.Ammo`))
    (bind _output_get (set `self.Mag` _asbp_ammo_base))
    (`self.Drop` _output_get (`/Game/Blueprints/Interaction/BP_BaseInteractable.GrabPhys` _output_get))
    (bind _basemesh (`/Game/Blueprints/Interaction/BP_BaseInteractable.BaseMesh` _output_get))
    (`PrimitiveComponent.SetSimulatePhysics` _basemesh false)
    (`PrimitiveComponent.SetCollisionEnabled` _basemesh "NoCollision")
    (`self.K2_AttachToComponent` _output_get (`self.MagLoc`) "None" "SnapToTarget" "SnapToTarget" "SnapToTarget" true)))

(event `self.Mag_Trigger.OnComponentEndOverlap`
  (params (OverlappedComponent :type "PrimitiveComponent Object Reference") (OtherActor :type "Actor Object Reference") (OtherComp :type "PrimitiveComponent Object Reference") (OtherBodyIndex :type Integer))
  (bind _mag (`self.Mag`))
  ;[1 1 1] Detach Mag
  (bind _asbp_ammo_base (cast `/Game/Blueprints/Interaction/Weapons/Ranged/Ammo/BP_AmmoBase` OtherActor))
  (if (== (`/Game/Blueprints/Interaction/Weapons/Ranged/Ammo/BP_AmmoBase.AmmoType` _asbp_ammo_base) (`self.Ammo`))
    (`self.K2_DetachFromActor` _mag "KeepWorld" "KeepWorld" "KeepWorld")
    (`/Engine/EditorBlueprintResources/StandardMacros.IsValid` _mag
      (:`Is Valid`
        (set `self.Mag` null)))))

(fn `Fire`
  (returns (OutHit :type "HitResult Structure") (ReturnValue :type Boolean))
  (bind _muzzleloc (`self.MuzzleLoc`))
  (bind _mag (`self.Mag`))
  (bind _returnvalue (`SceneComponent.K2_GetComponentLocation` _muzzleloc))
  (if (> (`/Game/Blueprints/Interaction/Weapons/Ranged/Ammo/BP_AmmoBase.AmmoAmount` (`self.Mag`)) 0)
    (`self.FireFX`)
    (bind _result (`/Engine/EditorBlueprintResources/StandardMacros.DecrementInt` (`/Game/Blueprints/Interaction/Weapons/Ranged/Ammo/BP_AmmoBase.AmmoAmount` _mag))
      (:`  `
        (set `/Game/Blueprints/Interaction/Weapons/Ranged/Ammo/BP_AmmoBase.AmmoAmount` _result _mag)
        (bind (_outhit _returnvalue_2) (`KismetSystemLibrary.LineTraceSingle` :`Start` _returnvalue :`End` (+ (* (`SceneComponent.GetForwardVector` _muzzleloc) (`self.FireRange`)) _returnvalue) :`TraceChannel` "TraceTypeQuery1" :`bTraceComplex` true :`DrawDebugType` "ForDuration"))
        (return _outhit _returnvalue_2)))))

(fn `FireFX`
  (`GameplayStatics.SpawnEmitterAttached` (`self.MuzzleFlash`) (`self.MuzzleLoc`) "None" (0.0 0.0 0.0) (struct) (1.0 1.0 1.0) "SnapToTarget")
  (`GameplayStatics.SpawnSoundAttached` (`self.FireSoundFX`) (`self.MuzzleLoc`) "None" (0.0 0.0 0.0) (struct) "KeepRelativeOffset" false 1.0 1.0 0.0 null null))

(fn `RotateWeapon`
  (bind _secondaryhand (`self.SecondaryHand`))
  (`/Engine/EditorBlueprintResources/StandardMacros.IsValid` _secondaryhand
    (:`Is Valid`
      (`SceneComponent.K2_SetWorldRotation` (`self.BaseMesh`) (`KismetMathLibrary.FindLookAtRotation` (`self.K2_GetActorLocation` (`self.PrimHolding`)) (`self.K2_GetActorLocation` _secondaryhand)) false false))))

(fn `UserConstructionScript`
  (`parent.UserConstructionScript`))