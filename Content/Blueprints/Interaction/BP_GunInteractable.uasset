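; Interactable gun that fires a pistol shot on Use, with magazine attachment through a Box overlap.
; On overlap, if the overlapped component equals Mag, it casts the other actor to a magazine and snaps it to MagLoc, otherwise printing "No".
; With a chambered round, Pistol decrements magazine ammo, runs an unused-result debug trace and plays sound.
; Otherwise, ContainMagazine, never set here, gates chambering; AmmoInChamber never clears.
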(event `/Game/Blueprints/FunctionsAndInterfaces/BP_InteractionInterface.Use`
  (`self.Pistol`))

(event `self.Box.OnComponentBeginOverlap`
  (params (OverlappedComponent :type "PrimitiveComponent Object Reference") (OtherActor :type "Actor Object Reference") (OtherComp :type "PrimitiveComponent Object Reference") (OtherBodyIndex :type Integer) (bFromSweep :type Boolean) (SweepResult :type "HitResult Structure (by ref)"))
  (if (== OverlappedComponent (`self.Mag`))
    (set `self.Mag` (cast `/Game/Blueprints/Interaction/BP_MagazineInteractable` OtherActor :!pure true))
    (`self.K2_AttachToComponent` (`self.Mag`) (`self.MagLoc`) "None" "SnapToTarget" "SnapToTarget" "KeepWorld" true)
    (else
      (`KismetSystemLibrary.PrintString` "No" false))))

(fn `Pistol`
  (bind _mag (`self.Mag`))
  (bind _mag_2 (`self.Mag`))
  (if (`self.AmmoInChamber`)
    (set `/Game/Blueprints/Interaction/BP_MagazineInteractable.Ammo` (- (`/Game/Blueprints/Interaction/BP_MagazineInteractable.Ammo` _mag_2) 1) _mag_2)
    (`KismetSystemLibrary.LineTraceSingle` :`TraceChannel` "TraceTypeQuery1" :`DrawDebugType` "ForOneFrame")
    (`GameplayStatics.SpawnSoundAttached` null (`self.Box`) "None" (0.0 0.0 0.0) (struct) "KeepRelativeOffset" false 1.0 1.0 0.0 null null)
    (elif (`self.ContainMagazine`)
      (set `self.AmmoInChamber` true)
      (set `/Game/Blueprints/Interaction/BP_MagazineInteractable.Ammo` (- (`/Game/Blueprints/Interaction/BP_MagazineInteractable.Ammo` _mag) 1) _mag)
      (`GameplayStatics.PlaySoundAtLocation` null (0.0 0.0 0.0) (struct) 1.0 1.0 0.0 null null null))))

(fn `UserConstructionScript`
  (`parent.UserConstructionScript`))