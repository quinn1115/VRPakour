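; BP_Player is a VR player character that handles locomotion and physical jumping.
; The MoveForward axis moves it along the left motion controller's forward vector, so the hand steers movement.
; Each tick it compares the replicated VR camera's world Z to InitialHeight plus a small margin, calling Jump above that threshold and StopJumping otherwise.
; InitialHeight is read but never assigned in these graphs.
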(event `InputAxis|MoveForward`
  (params (AxisValue :type "Float (single-precision)"))
  ;[1 0.04674 0.7772] Movement Controller
  (`self.AddMovementInput` (`SceneComponent.GetForwardVector` (`self.LeftMotionController`)) AxisValue))

(event `self.ReceiveTick`
  (params (DeltaSeconds :type "Float (single-precision)"))
  (bind (_returnvalue_x _returnvalue_y _returnvalue_z) (`KismetMathLibrary.BreakVector` (`SceneComponent.K2_GetComponentLocation` (`self.VRReplicatedCamera`))))
  ;[1 0 0.7268] Jumping VR
  (if (> _returnvalue_z (+ (`self.InitialHeight`) 15.0))
    (`self.Jump`)
    (else
      (`self.StopJumping`))))

(fn `UserConstructionScript`)