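; BP_MotionController is a player motion-controller actor that grabs and drops BP_BaseInteractable items through a physics handle.
; Each tick, the PHMC handle's target follows the motion controller's world transform.
; Grab picks the nearest interactable overlapping the sphere and sends it a grab message, or drops a held ToggleGrab item.
; Drop messages the held item and clears state; the old overlap-based detection is disconnected.
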(event `self.ReceiveTick`
  (params (DeltaSeconds :type "Float (single-precision)"))
  (bind (_returnvalue_location _returnvalue_rotation) (`KismetMathLibrary.BreakTransform` (`SceneComponent.K2_GetComponentToWorld` (`self.MotionController`))))
  ;[0.3734 1 0] Target Loc Rot
  (`PhysicsHandleComponent.SetTargetLocationAndRotation` (`self.PH_MC`) _returnvalue_location _returnvalue_rotation))

(event `self.Sphere.OnComponentBeginOverlap`
  (params (OverlappedComponent :type "PrimitiveComponent Object Reference") (OtherActor :type "Actor Object Reference") (OtherComp :type "PrimitiveComponent Object Reference") (OtherBodyIndex :type Integer) (bFromSweep :type Boolean) (SweepResult :type "HitResult Structure (by ref)"))
  ;[1 0.01805 0] Get Near Item(OLD)
)

(event `self.Sphere.OnComponentEndOverlap`
  (params (OverlappedComponent :type "PrimitiveComponent Object Reference") (OtherActor :type "Actor Object Reference") (OtherComp :type "PrimitiveComponent Object Reference") (OtherBodyIndex :type Integer))
  ;[1 0.01805 0] Get Near Item(OLD)
)

(fn `Drop`
  (if (`self.GrabbingItem`)
    (message `/Game/Blueprints/FunctionsAndInterfaces/BP_InteractionInterface.DropItem` (`self.HoldingItem`) (`self.PH_MC`) self)
    (set `self.GrabbingItem` false)
    (set `self.HoldingItem` null)))

(fn `GetNearestItem`
  (returns (`Nearest Actor` :type "Actor Object Reference"))
  (locals (NearDist :type "Float (double-precision)" :default 10000.0) (NearestItem :type "Actor Object Reference"))
  (bind _sphere (`self.Sphere`))
  (for _array_element (`PrimitiveComponent.GetOverlappingActors` _sphere "/Game/Blueprints/Interaction/BP_BaseInteractable.BP_BaseInteractable_C")
    (bind _returnvalue (`KismetMathLibrary.VSize` (- (`self.K2_GetActorLocation` _array_element) (`SceneComponent.K2_GetComponentLocation` _sphere))))
    (if (< _returnvalue (`local.NearDist`))
      (set `local.NearestItem` _array_element)
      (set `local.NearDist` _returnvalue)))
  (return (`local.NearestItem`)))

(fn `Grab`
  (if (`self.GrabbingItem`)
    (if (`/Game/Blueprints/Interaction/BP_BaseInteractable.ToggleGrab` (cast `/Game/Blueprints/Interaction/BP_BaseInteractable` (`self.HoldingItem`) :!pure true))
      (`self.Drop`))
    (else
      (bind _nearest_actor (`self.GetNearestItem`))
      (`/Engine/EditorBlueprintResources/StandardMacros.IsValid` _nearest_actor
        (:`Is Valid`
          (bind _output_get (set `self.HoldingItem` _nearest_actor))
          (message `/Game/Blueprints/FunctionsAndInterfaces/BP_InteractionInterface.GrabItem` _output_get (`self.PH_MC`) self)
          (set `self.GrabbingItem` true))))))

(fn `UserConstructionScript`)