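; VR player character Blueprint with motion-controller-directed movement, double jump and wall running.
; Forward input follows the left controller's facing, while left trigger presses launch upward through a DoN, reset on landing or wall contact.
; Wall collider overlap plays a timeline that, while the trigger is held, zeroes gravity, constrains movement horizontally and pushes along the camera's initial forward.
; Release or overlap end clears the constraint and sets gravity from the actor's WallRun tag.
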(event `InputAxis|MoveForward`
  (params (AxisValue :type "Float (single-precision)"))
  ;[1 0.04674 0.7772] Movement Controller
  (`self.AddMovementInput` (`SceneComponent.GetForwardVector` (`self.LeftMotionController`)) AxisValue))

(event `self.ReceiveTick`
  (params (DeltaSeconds :type "Float (single-precision)"))
  ;[1 0 0.7268] Jumping VR
)

(event `self.ReceiveBeginPlay`
  ;[1 1 1] Begin Play
  (`MovementComponent.SetPlaneConstraintEnabled` (`self.VRMovementReference`) true))

(event `self.OnLanded`
  (params (Hit :type "HitResult Structure (by ref)"))
  ;[1 1 1] Double Jump
  (goto _label :!via `Reset`))

(event `Key|MotionController_Left_Trigger`
  (params (Key :type "Key Structure"))
  ;[1 1 1] Double Jump
  (:`Pressed`
    (bind _counter (`/Engine/EditorBlueprintResources/StandardMacros.Do N` 2 :!label _label)
      (:`Exit`
        (switch `int` _counter
          (:`1`
            _)
          (:`2`
            _))
        (`self.LaunchCharacter` (0.0 0.0 420.0) false true))))
  (:`Released`
    (`self.StopJumping`)))

(event `self.WallDetectionCollider.OnComponentBeginOverlap`
  (params (OverlappedComponent :type "PrimitiveComponent Object Reference") (OtherActor :type "Actor Object Reference") (OtherComp :type "PrimitiveComponent Object Reference") (OtherBodyIndex :type Integer) (bFromSweep :type Boolean) (SweepResult :type "HitResult Structure (by ref)"))
  (bind _vrmovementreference (`self.VRMovementReference`))
  (bind _vrmovementreference_2 (`self.VRMovementReference`))
  (`|ExecutionSequence`
    (:`then_0`
      (goto _label :!via `Reset`))
    (:`then_1`
      (set `self.PlayerDir` (`SceneComponent.GetForwardVector` (`self.VRReplicatedCamera`)))
      (if true
        (set `self.OnWall` true)
        (`Timeline|WallRun` :!label _label_2
          (:`Update`
            (if (> (`PlayerController.GetInputKeyTimeDown` (`GameplayStatics.GetPlayerController` 0) "MotionController_Left_Trigger") 0.0)
              (if (`self.OnWall`)
                (set `CharacterMovementComponent.GravityScale` 0.0 _vrmovementreference)
                (`MovementComponent.SetPlaneConstraintNormal` _vrmovementreference (0.0 0.0 1.0))
                (`CharacterMovementComponent.AddForce` _vrmovementreference (* (`self.PlayerDir`) 2000.0))
                (else
                  (set `CharacterMovementComponent.GravityScale` (`KismetMathLibrary.Conv_BoolToDouble` (`self.ActorHasTag` (stale `self.WallDetectionCollider.OnComponentEndOverlap` OtherActor) "WallRun")) _vrmovementreference_2 :!label _label_3)
                  (`MovementComponent.SetPlaneConstraintNormal` _vrmovementreference_2 (0.0 0.0 0.0))
                  (set `self.OnWall` false)))
              (else
                (goto _label_3)))))))))

(event `self.WallDetectionCollider.OnComponentEndOverlap`
  (params (OverlappedComponent :type "PrimitiveComponent Object Reference") (OtherActor :type "Actor Object Reference") (OtherComp :type "PrimitiveComponent Object Reference") (OtherBodyIndex :type Integer))
  (`|ExecutionSequence`
    (:`then_0`
      (goto _label_2 :!via `Stop`))
    (:`then_1`
      (if true
        (goto _label_3)))))

(fn `UserConstructionScript`)