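; BP_Reggie is a two-legged AI actor with procedural walking and an idle body offset driven by a timeline.
; Tick flip-flops between the legs each frame, lifting any foot that drifts too far from its reference point and line-tracing a new foothold.
; MoveLeg interpolates each foot toward its target.
; The head look-at rotation is never executed, and Explode simply destroys the actor.
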(event `self.ReceiveBeginPlay`
  (set `self.NewLocRight` (`SceneComponent.K2_GetComponentLocation` (`self.RestPosR`)))
  (set `self.NewLocLeft` (`SceneComponent.K2_GetComponentLocation` (`self.RestPosL`)))
  (bind (_direction _idle) (`Timeline|Idle` :!via `PlayFromStart`)
    (:`Update`
      (set `self.BodyLoc` (- _idle (0.0 0.0 100.0))))))

(event `self.ReceiveTick`
  (params (DeltaSeconds :type "Float (single-precision)"))
  (bind _footlocl (`self.FootLocL`))
  (bind _footlocr (`self.FootLocR`))
  (`|ExecutionSequence`
    (:`then_1`
      (`/Engine/EditorBlueprintResources/StandardMacros.DoOnce` false
        (:`Completed`
          ;[1 1 1] WalkRight
          (`self.MoveLegUp` _footlocr 50.0 :!label _label)
          (bind _newlocation (`self.TraceNewLoc` (`self.FSL_Right`)))
          (set `self.NewLocRight` _newlocation)
          (goto _label_2 :!via `Reset`))))
    (:`then_2`
      (`/Engine/EditorBlueprintResources/StandardMacros.FlipFlop`
        (:`A`
          (`|ExecutionSequence`
            (:`then_0`
              (if (> (`KismetMathLibrary.VSize` (- (`SceneComponent.K2_GetComponentLocation` (`self.FootLocR`)) (`SceneComponent.K2_GetComponentLocation` (`self.DistPosR`)))) 200.0)
                (goto _label)))
            (:`then_1`
              (`/Engine/EditorBlueprintResources/StandardMacros.DoOnce` false :!label _label_2
                (:`Completed`
                  (`KismetSystemLibrary.Delay` 2.0)
                  (`self.MoveLeg` _footlocr (`self.NewLocRight`) DeltaSeconds :!label _label_3))))
            (:`then_2`
              (goto _label_3))))
        (:`B`
          ;[1 1 1] Walk Left
          (`|ExecutionSequence`
            (:`then_0`
              (if (> (`KismetMathLibrary.VSize` (- (`SceneComponent.K2_GetComponentLocation` (`self.FootLocL`)) (`SceneComponent.K2_GetComponentLocation` (`self.DistPosL`)))) 200.0)
                (`self.MoveLegUp` _footlocl 50.0)
                (bind _newlocation_2 (`self.TraceNewLoc` (`self.FSL_Left`)))
                (set `self.NewLocLeft` _newlocation_2)
                (goto _label_4 :!via `Reset`)))
            (:`then_1`
              (`/Engine/EditorBlueprintResources/StandardMacros.DoOnce` false :!label _label_4
                (:`Completed`
                  (`KismetSystemLibrary.Delay` 2.0)
                  (`self.MoveLeg` _footlocl (`self.NewLocLeft`) DeltaSeconds :!label _label_5))))
            (:`then_2`
              (goto _label_5))))))))

(fn `Explode`
  (`self.K2_DestroyActor`))

(fn `LookAtActor`
  (params (Enemy :type "Actor Object Reference"))
  (returns (ReturnValue :type "Rotator Structure"))
  (return (`KismetMathLibrary.FindLookAtRotation` (`SceneComponent.GetSocketLocation` (`self.Mesh`) "Head") (`self.K2_GetActorLocation` Enemy))))

(fn `MoveLeg`
  (params (FootLoc :type "SceneComponent Object Reference") (NewLoc :type "Vector Structure") (DeltaTime :type "Float (double-precision)"))
  (`SceneComponent.K2_SetWorldLocation` FootLoc (`KismetMathLibrary.VInterpTo` (`SceneComponent.K2_GetComponentLocation` FootLoc) (`KismetMathLibrary.MakeVector` NewLoc_X NewLoc_Y (+ NewLoc_Z 10.0)) DeltaTime 10.0) false false))

(fn `MoveLegUp`
  (params (Foot :type "SceneComponent Object Reference") (Amount :type "Float (double-precision)"))
  (`SceneComponent.K2_SetWorldLocation` Foot (+ (`SceneComponent.K2_GetComponentLocation` Foot) (`KismetMathLibrary.MakeVector` 0.0 0.0 Amount)) false false))

(fn `TraceNewLoc`
  (params (StartLoc :type "SceneComponent Object Reference"))
  (returns (NewLocation :type "Vector Structure"))
  (bind _returnvalue (`SceneComponent.K2_GetComponentLocation` StartLoc))
  (bind _outhit (`KismetSystemLibrary.LineTraceSingle` _returnvalue (+ (* (`SceneComponent.GetForwardVector` StartLoc) 500.0) _returnvalue) "TraceTypeQuery1"))
  (return (`.Location` (`GameplayStatics.BreakHitResult` _outhit))))

(fn `UserConstructionScript`)